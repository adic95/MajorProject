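; VR player pawn that handles movement, camera rotation, firing and distance grabbing, using floor-level tracking.
; Tick feeds movement and look axes into Move and RotateCamera, then passes through a Gate that calls ShootCamera every frame while Fire is held.
; The B key triggers GrabFromDistance with the camera and prints a debug string.
; A SetWeaponTransform call is left unconnected and never runs.
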(event EventBeginPlay
  (Class|HeadMountedDisplayFunctionLibrary|SetTrackingOrigin "Floor"))

(event EventTick
  (params (DeltaSeconds :type Float%20%28single-precision%29))
  ;[1 1 1] Basic Player Input
  (Utilities|FlowControl|Sequence
    (:then_0
      (Class|FPSPlayerPawn|Move (Math|Vector2D|MakeVector2D (Input|AxisValues|GetMoveRight) (Input|AxisValues|GetMoveForward)))
      (Class|FPSPlayerPawn|RotateCamera (Math|Vector2D|MakeVector2D (Input|AxisValues|GetTurn) (Input|AxisValues|GetLookUp))))
    (:then_1
      ;[1 1 1] Firing
      (Utilities|FlowControl|Gate true
        (:Exit
          (Class|FPSPlayerPawn|ShootCamera))))))

(event Input|ActionEvents|InputActionFire
  (params (Key :type Key%20Structure))
  ;[1 1 1] Firing
  (:Pressed
    (Utilities|FlowControl|Gate true) ; enters at Open
  )
  (:Released
    (Utilities|FlowControl|Gate true) ; enters at Close
  ))

(event Input|KeyboardEvents|B
  (params (Key :type Key%20Structure))
  (:Pressed
    (Class|FPSPlayerPawn|GrabfromDistance (Variables|Default|GetCamera))
    (Development|PrintString "Hello")))

(fn ConstructionScript)