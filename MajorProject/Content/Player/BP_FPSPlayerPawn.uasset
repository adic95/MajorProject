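; First-person player pawn that handles movement, camera look, weapon firing, grabbing and throwing, with a floor-level tracking origin.
; Tick feeds input axes into movement and rotation, and fires every frame while a Gate held open by the Fire input allows it.
; Grab pulls from a distance to the right hand, throw records positions on press and releases afterwards, and mesh overlaps call Collide.
; BeginPlay creates the HUD widget, whose kill score the F key increments.
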(event OnComponentBeginOverlap(Mesh)
  (params (OverlappedComponent :type Primitive%20Component%20Object%20Reference) (OtherActor :type Actor%20Object%20Reference) (OtherComp :type Primitive%20Component%20Object%20Reference) (OtherBodyIndex :type Integer) (bFromSweep :type Boolean) (SweepResult :type Hit%20Result%20Structure%20%28by%20ref%29))
  (Class|FPSPlayerPawn|Collide OtherComp))

(event EventBeginPlay
  (Class|HeadMountedDisplayFunctionLibrary|SetTrackingOrigin "Floor")
  (bind _returnvalue (UserInterface|CreateWidget "/Game/UI/BP_Widget.BP_Widget_C"))
  (bind _output_get (Variables|Default|SetWidget _returnvalue))
  (UserInterface|Viewport|AddtoViewport _output_get 0))

(event EventTick
  (params (DeltaSeconds :type Float%20%28single-precision%29))
  ;[1 1 1] Basic Player Input
  (Utilities|FlowControl|Sequence
    (:then_0
      (Class|FPSPlayerPawn|Move (Math|Vector2D|MakeVector2D (Input|AxisValues|GetMoveRight) (Input|AxisValues|GetMoveForward)))
      (Class|FPSPlayerPawn|RotateCamera (Math|Vector2D|MakeVector2D (Input|AxisValues|GetTurn) (Input|AxisValues|GetLookUp))))
    (:then_1
      ;[1 1 1] Firing
      (Utilities|FlowControl|Gate true
        (:Exit
          (Class|FPSPlayerPawn|ShootWeapon))))))

(event Input|ActionEvents|InputActionFire
  (params (Key :type Key%20Structure))
  ;[1 1 1] Firing
  (:Pressed
    (Utilities|FlowControl|Gate true) ; enters at Open
  )
  (:Released
    (Utilities|FlowControl|Gate true) ; enters at Close
  ))

(event Input|ActionEvents|InputActionGrabWeapon
  (params (Key :type Key%20Structure))
  (:Pressed
    (Class|FPSPlayerPawn|GrabfromDistance (Variables|Default|GetRightHandMesh))
    (Development|PrintString "Hello")))

(event Input|ActionEvents|InputActionThrowWeapon
  (params (Key :type Key%20Structure))
  (:Pressed
    (Class|FPSPlayerPawn|RecordPositions))
  (:Released
    (Class|FPSPlayerPawn|ThrowWeapon)))

(event Input|KeyboardEvents|F
  (params (Key :type Key%20Structure))
  (:Pressed
    (Default|AddKillScore (Variables|Default|GetWidget))))

(fn ConstructionScript)